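; Audio visualizer Blueprint that plays a 2D sound on BeginPlay and analyzes its frequency spectrum and amplitude each Tick.
; Each analysis samples the sound wave at current game time over the frame's delta, normalizing bands to 0–1 against running extremes.
; A buffer pass stores rising frequency peaks and sets decrease rates, but never applies the decay or updates amplitude buffers.
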(event `self.ReceiveBeginPlay`
  (`GameplayStatics.PlaySound2D` (`self.Sound`) 1.0 1.0 0.0 null null)
  (`KismetArrayLibrary.Array_Resize` (`self.FreqSpectrum`) (`self.N°FreqBands`))
  (`KismetArrayLibrary.Array_Resize` (`self.AmpSpectrum`) (`self.N°AmpBands`))
  (`KismetArrayLibrary.Array_Resize` (`self.FreqBuffer`) (`self.N°FreqBands`))
  (`KismetArrayLibrary.Array_Resize` (`self.AmpBuffer`) (`self.N°AmpBands`))
  (`KismetArrayLibrary.Array_Resize` (`self.FreqBufferDecrease`) (`self.N°FreqBands`))
  (`KismetArrayLibrary.Array_Resize` (`self.AmpBufferDecrease`) (`self.N°AmpBands`)))

(event `self.ReceiveTick`
  (params (DeltaSeconds :type "Float (single-precision)"))
  (`self.CalculateFrequency&Amplitude` DeltaSeconds)
  (`self.CalculateAudioBuffer`))

(fn `CalculateAudioBuffer`
  (for (_array_element _array_index) (`self.FreqSpectrum`)
    (if (> _array_element (`|GetArrayItem` (`self.FreqBuffer`) _array_index))
      (`KismetArrayLibrary.Array_Set` (`self.FreqBuffer`) _array_index _array_element)
      (`KismetArrayLibrary.Array_Set` (`self.FreqBufferDecrease`) _array_index (/ 1.0 (`self.BufferAmount`))))))

(fn `CalculateFrequency&Amplitude`
  (params (Delta :type "Float (double-precision)"))
  (locals (Interval :type "Float (double-precision)") (MaxAmpProfile :type "Float (double-precision)") (MaxFreqProfile :type "Float (double-precision)") (MinFreqProfile :type "Float (double-precision)"))
  ;[1 1 1] Calculates Audio Frequency Spectrum & Amp Spectrum Range From 0...1
  (bind _output_get (set `local.Interval` Delta))
  (bind _outspectrum (`SoundVisualizationStatics.CalculateFrequencySpectrum` (`self.Sound`) 0 (`KismetSystemLibrary.GetGameTimeInSeconds`) _output_get (`self.N°FreqBands`)))
  (for (_array_element _array_index) _outspectrum
    (if (> _array_element (`local.MaxFreqProfile`))
      (set `local.MaxFreqProfile` _array_element))
    (if (< _array_element (`local.MinFreqProfile`))
      (set `local.MinFreqProfile` _array_element))
    (`KismetArrayLibrary.Array_Set` (`self.FreqSpectrum`) _array_index (`KismetMathLibrary.MapRangeClamped` _array_element (`local.MinFreqProfile`) (`local.MaxFreqProfile`) 0.0 1.0)))
  (bind _outamplitudes (`SoundVisualizationStatics.GetAmplitude` (`self.Sound`) 0 (`KismetSystemLibrary.GetGameTimeInSeconds`) (`local.Interval`) (`self.N°AmpBands`)))
  (for (_array_element_2 _array_index_2) _outamplitudes
    (if (> _array_element_2 (`local.MaxAmpProfile`))
      (set `local.MaxAmpProfile` _array_element_2))
    (`KismetArrayLibrary.Array_Set` (`self.AmpSpectrum`) _array_index_2 (`KismetMathLibrary.MapRangeClamped` _array_element_2 0.0 (`local.MaxAmpProfile`) 0.0 1.0))))

(fn `UserConstructionScript`)